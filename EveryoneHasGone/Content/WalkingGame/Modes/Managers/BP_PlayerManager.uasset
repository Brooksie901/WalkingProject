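; Player manager for the walking game that spawns the player character and controls when it accepts input, through events the GameMode calls.
; Init spawns BP_WalkingCharacter at the last PlayerStart found, possesses it with player controller 0 and disables its input.
; StartInput re-enables that input when the game starts.
; The PlayerStart search fails only on an invalid entry, so an empty level still reports success.
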(event EventBeginPlay
  (|CallParentFunction) ; This node is disabled and will not be called.\nDrag off pins to build functionality.
)

(event Collision|EventActorBeginOverlap
  (params (OtherActor :type Actor%20Object%20Reference))
  (|CallParentFunction OtherActor) ; This node is disabled and will not be called.\nDrag off pins to build functionality.
)

(event EventTick
  (params (DeltaSeconds :type Float%20%28single-precision%29))
  (|CallParentFunction DeltaSeconds) ; This node is disabled and will not be called.\nDrag off pins to build functionality.
)

(event EventInit
  ;[1 1 1] Called On Init on GameMode
  (CallFunction|SpawnCharacter))

(event EventStartInput
  ;[1 1 1] Called On Start Game on GameMode
  (CallFunction|GiveInput))

(fn ConstructionScript
  (|CallParentFunction))

(fn SpawnCharacter
  (bind _returnvalue (Game|GetPlayerController 0))
  (bind (_sucess _playerstarttransform) (CallFunction|FindPlayerStart))
  (if _sucess
    (bind _returnvalue_2 (Game|SpawnActorfromClass "/Game/WalkingGame/Character/BP_WalkingCharacter.BP_WalkingCharacter_C" _playerstarttransform "Undefined" "MultiplyWithRoot" 0 0))
    (bind _output_get (Variables|Default|SetPlayerCharacterRef _returnvalue_2))
    (Pawn|Possess _returnvalue _output_get)
    (Input|DisableInput _output_get _returnvalue)
    (else
      (Development|PrintString "Player Start Not Found" true true "(R=1.000000,G=0.100782,B=0.000000,A=1.000000)"))))

(fn FindPlayerStart
  (bind _outactors (Actor|GetAllActorsOfClass "/Script/Engine.PlayerStart"))
  (bind _array_element (Utilities|Array|ForEachLoopwithBreak _outactors)
    (:LoopBody
      (Utilities|IsValid _array_element
        (:Is%20Valid
          (Variables|Default|SetPlayerStartTransform (Transformation|GetActorTransform _array_element)))
        (:Is%20Not%20Valid
          (return false ""))))
    (:Completed
      (return true (Variables|Default|GetPlayerStartTransform)))))

(fn GiveInput
  (bind _playercharacterref (Variables|Default|GetPlayerCharacterRef))
  (Utilities|IsValid _playercharacterref
    (:Is%20Valid
      (Input|EnableInput _playercharacterref (Game|GetPlayerController 0)))
    (:Is%20Not%20Valid
      (Development|PrintString "Player Character Not Valid"))))