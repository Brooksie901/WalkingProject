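; Game mode for the walking game that runs a linear state flow from initialization to game end.
; ChangeGameState dispatches each state to its event, which advances to the next immediately, so BeginPlay runs straight through to a "GAME ENDED" print.
; Initialization finds the player and puzzle managers in the level and sends them an init message, printing an error if one is missing.
; StartGame sends the player manager a start-input message.
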(event Custom|Initiliaztion
  (CallFunction|SetUpManager "/Game/WalkingGame/Modes/Managers/BP_PlayerManager.BP_PlayerManager_C")
  (CallFunction|SetUpManager "/Game/WalkingGame/Modes/Managers/BP_PuzzleManager.BP_PuzzleManager_C")
  (CallFunction|ChangeGameState "NewEnumerator1"))

(event Custom|Pre%20Game
  (CallFunction|ChangeGameState "NewEnumerator2"))

(event Custom|Start%20Game
  (CallFunction|GetManager "/Game/WalkingGame/Modes/Managers/BP_PlayerManager.BP_PlayerManager_C")
  (CallFunction|ChangeGameState "NewEnumerator3"))

(event Custom|End%20Game
  (Development|PrintString "GAME ENDED"))

(event EventBeginPlay
  (CallFunction|ChangeGameState "NewEnumerator0"))

(fn ConstructionScript)

(fn ChangeGameState
  (params (State :type Enum_GameStates%20Enum :default "NewEnumerator0"))
  (switch Utilities|FlowControl|Switch|SwitchonEnum_GameStates State
    (:NewEnumerator0
      (CallFunction|Initiliaztion))
    (:NewEnumerator1
      (CallFunction|PreGame))
    (:NewEnumerator2
      (CallFunction|StartGame))
    (:NewEnumerator3
      (CallFunction|EndGame))))

(fn SetUpManager
  (params (Manager%20Class%20Type :type BP%20Base%20Manager%20Class%20Reference))
  (bind _returnvalue (Actor|GetActorOfClass Manager%20Class%20Type))
  (bind _output_get (LocalVariables|SetTempManagerRef _returnvalue))
  (Utilities|IsValid _output_get
    (:Is%20Valid
      (Class|BPIInitalization|Init(Message) (LocalVariables|GetTempManagerRef)))
    (:Is%20Not%20Valid
      (Development|PrintString (Utilities|String|Append "Error: Manager of type (" (Utilities|GetClassDisplayName Manager%20Class%20Type) ") is not in level") true true "(R=1.000000,G=0.000000,B=0.016462,A=1.000000)"))))

(fn GetManager
  (params (Manager%20To%20Get :type BP%20Base%20Manager%20Class%20Reference))
  (bind _returnvalue (Actor|GetActorOfClass Manager%20To%20Get))
  (Class|BPIManagerCalls|StartInput(Message) _returnvalue))