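; BP_PillarTrigger is an interactable trigger that activates the message of a referenced pillar.
; Its Interact event prints the display name of the passed player reference, then passes through a DoOnce to call ActivatePillarMessage on PillarRef, so the pillar is activated only on the first interaction.
; BeginPlay, overlap and Tick are unused stubs, and the construction script only calls its parent.
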(event EventBeginPlay
  (|CallParentFunction) ; This node is disabled and will not be called.\nDrag off pins to build functionality.
)

(event Collision|EventActorBeginOverlap
  (params (OtherActor :type Actor%20Object%20Reference))
  (|CallParentFunction OtherActor) ; This node is disabled and will not be called.\nDrag off pins to build functionality.
)

(event EventTick
  (params (DeltaSeconds :type Float%20%28single-precision%29))
  (|CallParentFunction DeltaSeconds) ; This node is disabled and will not be called.\nDrag off pins to build functionality.
)

(event EventInteract
  (params (Player%20Ref :type Actor%20Object%20Reference))
  (Development|PrintString (Utilities|GetDisplayName Player%20Ref))
  (Utilities|FlowControl|DoOnce false
    (:Completed
      (Class|BPIPillar|ActivatePillar(Message) (Variables|Default|GetPillarRef)))))

(fn ConstructionScript
  (|CallParentFunction))