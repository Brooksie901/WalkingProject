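; BP_PillarWater is the water pillar in the walking game's pillar puzzle, reporting its activation to a puzzle manager.
; InitilizePuzzles stores the puzzle manager reference passed to it.
; ActivatePillar passes the pillar's PillarType to CheckPillarComplete on that manager, so the completion logic lives outside this Blueprint.
; It has no active BeginPlay, Tick or overlap logic, and its construction script only calls the parent.
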(event EventBeginPlay
  (|CallParentFunction) ; This node is disabled and will not be called.\nDrag off pins to build functionality.
)

(event Collision|EventActorBeginOverlap
  (params (OtherActor :type Actor%20Object%20Reference))
  (|CallParentFunction OtherActor) ; This node is disabled and will not be called.\nDrag off pins to build functionality.
)

(event EventTick
  (params (DeltaSeconds :type Float%20%28single-precision%29))
  (|CallParentFunction DeltaSeconds) ; This node is disabled and will not be called.\nDrag off pins to build functionality.
)

(event EventActivatePillar
  (Default|CheckPillarComplete (Variables|Default|GetPuzzle%20Manager%20Ref) (Variables|Default|GetPillarType)))

(event EventInitilizePuzzles
  (params (Puzzle%20Manager%20Ref :type BP%20Puzzle%20Manager%20Object%20Reference))
  (Variables|Default|SetPuzzle%20Manager%20Ref Puzzle%20Manager%20Ref))

(fn ConstructionScript
  (|CallParentFunction))